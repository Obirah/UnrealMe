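; Player controller for UnrealMe Kinect characters that starts the Kinect connection on BeginPlay and disconnects it on EndPlay.
; MultiUserSpawn, not called within this graph, fills an array with the player character plus five spawned characters, each with its own skeleton index.
; N cycles possession through that array, querying but ignoring whether the user is tracked.
; T shifts the player character's capsule sideways along Y.
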(event EventEndPlay
  (params (EndPlayReason :type EEndPlayReason%20Enum :default "ActorDestroyed"))
  (Class|UnrealMeKinectV2Connector|DisconnectKinect))

(event EventBeginPlay
  (if (not (Variables|Default|GetKinectInitialized))
    (Class|UnrealMeKinectV2Connector|InitializeKinect)
    (Variables|Default|SetKinectInitialized true)))

(event Input|KeyboardEvents|T
  (bind _returnvalue (Game|GetPlayerCharacter 0))
  (:Pressed
    (Transformation|SetWorldLocation (Variables|/Script/Engine.Character|GetCapsuleComponent _returnvalue) (+ (Transformation|GetActorLocation _returnvalue) "0,500.000000, 0") false)))

(event Input|KeyboardEvents|N
  (:Pressed
    (CallFunction|SwitchCharcterPossesion)))

(fn ConstructionScript)

(fn SwitchCharcterPossesion
  (Math|Integer|CompareInt (Variables|Default|GetCurrentUserView) 0
    (:>
      (Math|Integer|CompareInt (Variables|Default|GetCurrentUserView) 5 :!label _label
        (:>
          (Variables|Default|SetCurrentUserView 0))
        (:==
          _)
        (:<
          _)))
    (:==
      (goto _label))
    (:<
      (Variables|Default|SetCurrentUserView 0)))
  (bind _returnvalue (Class|UnrealMeKinectV2Connector|IsUserTracked (Variables|Default|GetCurrentUserView)))
  (if _returnvalue
    _
    (else
      _))
  (Pawn|Possess (Game|GetPlayerController 0) (Utilities|Array|Get(acopy) (Variables|Default|GetKinectCharacters) (Variables|Default|GetCurrentUserView)))
  (Math|Integer|CompareInt (Variables|Default|GetCurrentUserView) 5
    (:>
      (Variables|Default|SetCurrentUserView 0 :!label _label_2))
    (:==
      (goto _label_2))
    (:<
      (Variables|Default|SetCurrentUserView (+ (Variables|Default|GetCurrentUserView) 1))))
  (Variables|Default|SetCurrentCharacter (Utilities|Array|Get(acopy) (Variables|Default|GetKinectCharacters) (Variables|Default|GetCurrentUserView))))

(fn MultiUserSpawn
  (for _index (range 0 5)
    (Math|Integer|CompareInt _index 0
      (:>
        (bind _returnvalue (Game|SpawnActorfromClass "/Game/Character/UnrealMe/UnrealMeKinectCharacter.UnrealMeKinectCharacter_C" (Math|Conversions|ToTransform(Vector) (+ "0, 0, 0" (* "0,-100.000000, 0" (Math|Conversions|ToFloat(Integer) _index)))) false _index 0))
        (Utilities|Array|Add (Variables|Default|GetKinectCharacters) _returnvalue))
      (:==
        (Utilities|Array|Add (Variables|Default|GetKinectCharacters) (Game|GetPlayerCharacter 0)))))
  (Class|UnrealMeKinectV2Connector|InitializeKinect)
  (Variables|Default|SetKinectInitialized true))