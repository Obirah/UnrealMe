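; Player controller for the UnrealMe Kinect avatar, providing hotkeys to tune and debug body tracking.
; B toggles pure-rotation mode on the character's rotation embodiment AnimInstance, and right mouse sets the torso offset from a tracked joint position once Kinect is initialized.
; X, Y and Z each apply a quarter-turn offset rotation on a separate axis and print the result, while T shifts the character by a fixed world offset.
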(event Input|KeyboardEvents|X
  (:Pressed
    (bind _returnvalue (Class|UnrealMeKinectV2Connector|OffsetRotation 1 90))
    (Development|PrintString (Utilities|String|ToString(Integer) _returnvalue))))

(event Input|KeyboardEvents|Y
  (:Pressed
    (bind _returnvalue (Class|UnrealMeKinectV2Connector|OffsetRotation 2 90))
    (Development|PrintString (Utilities|String|ToString(Integer) _returnvalue))))

(event Input|KeyboardEvents|Z
  (:Pressed
    (bind _returnvalue (Class|UnrealMeKinectV2Connector|OffsetRotation 3 90))
    (Development|PrintString (Utilities|String|ToString(Integer) _returnvalue))))

(event Input|KeyboardEvents|B
  (:Pressed
    (bind _asunreal_me_kinect_character (Utilities|Casting|CastToUnrealMeKinectCharacter (Game|GetPlayerCharacter 0)))
    (bind _asunreal_me_kinect_rotation_embodiment (Utilities|Casting|CastToUnrealMeKinectRotationEmbodiment (Components|SkeletalMesh|GetAnimInstance _asunreal_me_kinect_character)))
    (if (Variables|/Game/Animations/UnrealMe/UnrealMeKinectRotationEmbodiment.UnrealMeKinectRotationEmbodiment_C|GetUsePureRotations _asunreal_me_kinect_rotation_embodiment)
      (Variables|/Game/Animations/UnrealMe/UnrealMeKinectRotationEmbodiment.UnrealMeKinectRotationEmbodiment_C|SetUsePureRotations _asunreal_me_kinect_rotation_embodiment false)
      (else
        (Variables|/Game/Animations/UnrealMe/UnrealMeKinectRotationEmbodiment.UnrealMeKinectRotationEmbodiment_C|SetUsePureRotations _asunreal_me_kinect_rotation_embodiment true)))))

(event Input|KeyboardEvents|T
  (:Pressed
    (Class|Actor|AddActorWorldTransform (Game|GetPlayerCharacter 0) (Math|Transform|MakeTransform "0,-500.000000,500.000000") false)))

(event Input|MouseEvents|RightMouseButton
  (:Pressed
    (if (Variables|Default|GetKinectInitialized)
      (Utilities|Casting|CastToUnrealMeKinectCharacter (Game|GetPlayerCharacter 0))
      (bind _returnvalue (Class|UnrealMeKinectV2Connector|GetJointPosition 7))
      (Class|UnrealMeKinectV2Connector|SetCurrentTorsoOffset _returnvalue))))

(fn ConstructionScript)